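; Player gameplay ability for the primary attack, activated by an event that supplies the target and attack speed.
; It turns the player toward the target and scales the montage play rate so one swing lasts 1/AttackSpeed seconds.
; On completion it ends successfully, then next tick sends an auto-attack event with the same target and speed to request another attack.
; Interruption or cancellation stops the montage and ends the ability as cancelled.
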(event Custom|RequestAutoAttack
  (Class|MPlayerAbility|SendGameplayEventtoOwner (Variables|Default|GetAutoAttackTag) (Utilities|Struct|MakeGameplayEventData "(TagName=\"\")" 0 (Variables|Default|GetTargetActor) 0 0 "()" "(GameplayTags=)" "(GameplayTags=)" (Variables|Default|GetAttackSpeed) "()")))

(event Ability|EventActivateAbilityFromEvent
  (params (EventData :type Gameplay%20Event%20Data%20Structure%20%28by%20ref%29))
  (bind _characterattackmontages (Variables|Default|GetCharacterAttackMontages))
  (bind _output_get (Variables|Default|SetAttackSpeed (.eventmagnitude EventData)))
  (bind _output_get_2 (Variables|Default|SetTargetActor (.target EventData)))
  (Class|MPlayerMovementComponent|FaceTargetActor (Class|MPlayerAbility|GetMPlayerMovementComponent) _output_get_2)
  (|PlayMontageandWaitProxy "None" _characterattackmontages (/ (Animation|GetPlayLength _characterattackmontages) (/ 1.0 _output_get)) "None" true 1.0 0.0 false
    (:OnCompleted
      (Class|MGameplayAbility|EndAbilityasSuccess true)
      (Class|KismetSystemLibrary|SetTimerforNextTickDelegate (delegate Custom|RequestAutoAttack)))
    (:OnInterrupted
      (Animation|Montage|MontageStop -1.0 :!label _label)
      (Class|MGameplayAbility|EndAbilityasCancelled true))
    (:OnCancelled
      (goto _label))))