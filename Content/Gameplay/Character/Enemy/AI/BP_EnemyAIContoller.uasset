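; Enemy AI controller that tracks the player through AI Perception and writes the TargetActor blackboard key.
; Sensing a Player-tagged actor cancels the tracking timer and sets it as the target.
; Any other perception update, including non-player stimuli, starts a TrackingTime timer whose StartTargetTimer event clears the target, giving a grace period.
; Possess only casts the pawn to MEnemyCharacterBase.
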(event OnTargetPerceptionUpdated(AIPerception)
  (params (Actor :type Actor%20Object%20Reference) (Stimulus :type AI%20Stimulus%20Structure))
  (if (and (Actor|ActorHasTag Actor "Player") (.bSuccessfullySensed (Utilities|Struct|BreakAIStimulus Stimulus)))
    (Utilities|Time|ClearandInvalidateTimerbyHandle (Variables|Default|GetTrackingTimer))
    (AI|Components|Blackboard|SetValueasObject (Variables|Default|GetBlackboard) (Variables|Default|GetTargetActor) Actor)
    (else
      (bind _returnvalue (Utilities|Time|SetTimerbyEvent (delegate Custom|StartTargetTimer) (Variables|Default|GetTrackingTime)))
      (Variables|Default|SetTrackingTimer _returnvalue))))

(event Custom|StartTargetTimer
  (AI|Components|Blackboard|SetValueasObject (Variables|Default|GetBlackboard) (Variables|Default|GetTargetActor) 0))

(event EventPossess
  (params (PossessedPawn :type Pawn%20Object%20Reference))
  (bind _asmenemy_character_base (Utilities|Casting|CastToMEnemyCharacterBase PossessedPawn)))

(fn ConstructionScript)